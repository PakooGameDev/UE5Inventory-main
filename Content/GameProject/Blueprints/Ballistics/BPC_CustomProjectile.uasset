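; Bullet ballistics component that simulates a whole trajectory at BeginPlay as stepped line traces, applying gravity and drag.
; On hit, a physical-material data table lookup gates penetration, though material resistance is passed as zero into the depth formula's divisor.
; A reverse trace finds the exit point, then decals are placed, speed drops and direction scatters.
; Ricochet logic is unconnected; optional debug lines are colored by speed.
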(event Custom|Ballistics
  (bind _index (Utilities|FlowControl|ForLoopwithBreak 0 (Variables|Default|GetTrajectoryStepCount) :!label _label)
    (:LoopBody
      (Variables|Default|SetDeltaTime (* _index (Variables|Default|GetTrajectoryTimeStep)))
      (Variables|Default|SetFirstPos (Variables|Default|GetLastPos))
      (Variables|Default|SetLastPos (+ (Variables|Default|GetFirstPos) (* (Variables|BulletParams|GetVelocity) (Variables|Default|GetDeltaTime))))
      (bind (_outhit _returnvalue) (Collision|LineTraceByChannel (Variables|Default|GetFirstPos) (Variables|Default|GetLastPos) "TraceTypeQuery1" false (Utilities|Array|MakeArray (Variables|Default|GetActorToIgnore)) "None" true "(R=1.000000,G=0.000000,B=0.000000,A=1.000000)" "(R=0.000000,G=1.000000,B=0.000000,A=1.000000)" 1e+01))
      (bind _output_get (Variables|Default|SetOut%20Hit _outhit))
      (Utilities|DrawLine _output_get)
      (if _returnvalue
        (if (CallFunction|WhethertoPenetrate (Variables|BulletParams|GetVelocity) (Variables|Default|GetOut%20Hit))
          (CallFunction|BulletHole (Variables|Default|GetOut%20Hit))
          (bind _hit (CallFunction|ComputeExitLocation (Variables|Default|GetOut%20Hit)))
          (if _hit
            (Variables|Default|SetActorToIgnore (.HitActor (Collision|BreakHitResult (Variables|Default|GetOut%20Hit))))
            (CallFunction|VaryTrajectory (* (.ImpactNormal (Collision|BreakHitResult (Variables|Default|GetOut%20Hit))) -1.0))
            (else
              (goto _label Break))))
        (else
          (Variables|BulletParams|SetVelocity (CallFunction|CalculateAcceleration (Variables|BulletParams|GetVelocity))))))))

(event EventBeginPlay
  (Variables|BulletParams|SetVelocity (* (Transformation|GetActorForwardVector (Components|GetOwner)) (* (Variables|BulletParams|GetBulletSpeed) 1e+02)))
  (Variables|Default|SetLastPos (Transformation|GetActorLocation (Components|GetOwner)))
  (CallFunction|Ballistics))

(fn ComputeExitLocation
  (params (HitResult :type Hit%20Result%20Structure))
  (bind (_bblockinghit _binitialoverlap _time _distance _location _impactpoint _normal _impactnormal _physmat _hitactor) (Collision|BreakHitResult HitResult))
  (bind _boxextent (Collision|GetActorBounds _hitactor true true))
  (bind _output_get (LocalVariables|SetDirection (Math|Vector|Normalize (Variables|BulletParams|GetVelocity))))
  (LocalVariables|SetTraceDistance (* (Math|Float|Max(Float) (.x _boxextent) (.y _boxextent) (.z _boxextent)) 2.0))
  (bind _output_get_2 (LocalVariables|SetTraceStart (+ (* _output_get (LocalVariables|GetTraceDistance)) _impactpoint)))
  (LocalVariables|SetTraceEnd (+ (* (LocalVariables|GetDirection) (* (LocalVariables|GetTraceDistance) -1.0)) _output_get_2))
  (bind (_outhit _returnvalue) (Collision|LineTraceByChannel (LocalVariables|GetTraceStart) (LocalVariables|GetTraceEnd) "TraceTypeQuery1" false (LocalVariables|GetIgnoreList) "None" true "(R=1.000000,G=0.996379,B=0.000000,A=1.000000)" "(R=0.000000,G=0.912769,B=1.000000,A=1.000000)" :!label _label))
  (if _returnvalue
    (if (!= (.HitActor (Collision|BreakHitResult _outhit)) _hitactor)
      (Utilities|Array|Add (LocalVariables|GetIgnoreList) (.HitActor (Collision|BreakHitResult _outhit)))
      (LocalVariables|SetTraceStart (.ImpactPoint (Collision|BreakHitResult _outhit)))
      (goto _label)
      (elif (> (Variables|Default|GetDepthOfPenetration) (Math|Vector|Distance(Vector) (.ImpactPoint (Collision|BreakHitResult _outhit)) _impactpoint))
        (CallFunction|BulletHole _outhit)
        (Variables|BulletParams|SetVelocity (CallFunction|CalculateAcceleration (* (- 1.0 (* (Math|Vector|Distance(Vector) (.ImpactPoint (Collision|BreakHitResult _outhit)) _impactpoint) 0.01)) (Variables|BulletParams|GetVelocity))))
        (Variables|Default|SetLastPos (.ImpactPoint (Collision|BreakHitResult _outhit)))
        (return true)
        (else
          (Variables|BulletParams|SetVelocity "0, 0, 0")
          (return false))))
    (else
      (return false))))

(fn WhethertoPenetrate
  (params (Velocity :type Vector) (Hit :type Hit%20Result%20Structure))
  (bind _returnvalue (Utilities|GetDataTableRow "/Game/GameProject/Blueprints/Ballistics/Data.Data" (Utilities|String|StringToName (Utilities|GetObjectName (.PhysMat (Collision|BreakHitResult Hit)))))
    (:then
      (bind _output_get (Variables|Default|SetDepthOfPenetration (CallFunction|CalculatePenetrationDepth Velocity 0.0 (Utilities|Struct|BreakPenetrationData _returnvalue))))
      (if (> _output_get 0.0)
        (return true)
        (else
          (return false))))
    (:RowNotFound
      (return false))))

(fn ComputeRicochet
  (params (Hit :type Hit%20Result%20Structure%20%28by%20ref%29))
  (bind (_bblockinghit _binitialoverlap _time _distance _location _impactpoint _normal _impactnormal) (Collision|BreakHitResult Hit))
  (bind _velocity (Variables|BulletParams|GetVelocity))
  (bind _returnvalue (Math|Vector|VectorLength _velocity))
  (return (+ _impactpoint _impactnormal) _impactnormal (Math|Vector|MirrorVectorbyNormal (* (Math|Vector|Normalize (Variables|BulletParams|GetVelocity)) (- _returnvalue (/ _returnvalue 2.0))) _impactnormal)))

(fn GetTraceColor
  (bind _bulletspeed (Variables|BulletParams|GetBulletSpeed))
  (bind _velocity (Variables|BulletParams|GetVelocity))
  (bind _returnvalue (Math|Vector|VectorLength _velocity))
  (bind _returnvalue_2 (* _bulletspeed 1e+02))
  (bind _returnvalue_3 (/ _returnvalue _returnvalue_2))
  (if (> _returnvalue_3 0.75)
    (return (Math|Color|Lerp(LinearColor) "(R=0.223228,G=0.000000,B=0.001518,A=1.000000)" "(R=0.005208,G=0.000029,B=0.000000,A=1.000000)" (- _returnvalue_3 0.75)))
    (elif (> _returnvalue_3 0.5)
      (return (Math|Color|Lerp(LinearColor) "(R=1.000000,G=0.577581,B=0.000000,A=1.000000)" "(R=0.223228,G=0.000000,B=0.001518,A=1.000000)" (- _returnvalue_3 0.5)))
      (elif (> _returnvalue_3 0.25)
        (return (Math|Color|Lerp(LinearColor) "(R=0.000000,G=1.000000,B=0.270498,A=1.000000)" "(R=1.000000,G=0.577581,B=0.000000,A=1.000000)" (- _returnvalue_3 0.25)))
        (else
          (return (Math|Color|Lerp(LinearColor) "(R=0.708376,G=1.000000,B=0.701102,A=1.000000)" "(R=0.000000,G=1.000000,B=0.270498,A=1.000000)" _returnvalue_3)))))))

(fn VaryTrajectory
  (params (SurfaceNormal :type Vector))
  (LocalVariables|SetInitialAnswer (* (Class|KismetMathLibrary|RandomUnitVectorinConeinRadians (Variables|BulletParams|GetVelocity) (Math|Float|MapRangeClamped (Math|Vector|VectorLength (Variables|BulletParams|GetVelocity)) 1e+04 1e+05 0.087266 0.174533)) (Math|Vector|VectorLength (Variables|BulletParams|GetVelocity))))
  (if (>= (CallFunction|AngleBetweenVectors SurfaceNormal (LocalVariables|GetInitialAnswer)) 9e+01)
    (Variables|BulletParams|SetVelocity (Math|Vector|RotateVector (LocalVariables|GetInitialAnswer) (* (Math|Rotator|Delta(Rotator) (Math|Rotator|MakeRotfromX SurfaceNormal) (Math|Rotator|MakeRotfromX (LocalVariables|GetInitialAnswer))) (- 1.0 (/ (CallFunction|AngleBetweenVectors SurfaceNormal (LocalVariables|GetInitialAnswer)) 9e+01)))))
    (else
      (Variables|BulletParams|SetVelocity (LocalVariables|GetInitialAnswer))))
  (return))

(fn BulletHole
  (params (HitResult :type Hit%20Result%20Structure))
  (bind _returnvalue (Rendering|Decal|SpawnDecalatLocation (Variables|BulletHole|GetDecal%20Material) (Variables|BulletHole|GetDecal%20Size) (.location HitResult) (Math|Rotator|MakeRotfromX (.impactnormal HitResult)) (Variables|BulletHole|GetDecalLifeSpan)))
  (Rendering|Components|Decal|SetFadeScreenSize _returnvalue (Variables|BulletHole|GetDecalFadeScreenSize)))

(fn AngleBetweenVectors
  (params (V1 :type Vector) (V2 :type Vector))
  (return (Class|KismetMathLibrary|DegAcos (Math|Vector|DotProduct (Math|Vector|Normalize V1) (Math|Vector|Normalize V2)))))

(fn CalculateAcceleration
  (params (InitialVelocity :type Vector))
  (return (+ InitialVelocity (* (- (* (Variables|Enviromental|GetGravity) (Variables|BulletParams|GetBulletMass)) (/ (* (Math|Vector|Normalize InitialVelocity) (Math|Vector|VectorLengthSquared InitialVelocity) (Variables|Enviromental|GetAirDensity) (Variables|BulletParams|GetCrossSection)) 4.0)) (Variables|Default|GetDeltaTime)))))

(fn CalculatePenetrationDepth
  (params (BulletVelocity :type Vector) (MaterialResistance :type Float%20%28double-precision%29) (MaterialDensity :type Float%20%28double-precision%29))
  (return (/ (* (Math|Vector|VectorLength BulletVelocity) (Variables|BulletParams|GetBulletMass)) (* MaterialResistance MaterialDensity))))